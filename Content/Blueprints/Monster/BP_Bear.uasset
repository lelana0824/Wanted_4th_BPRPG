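; BP_Bear is a bear monster that chases the player, takes damage and dies.
; A simple tick-driven state machine (Locomotion, Chase, Attack, Dead) sets walk speed on each transition.
; PawnSensing stores the player in the Blackboard and starts Chase, which ends beyond sight radius.
; BPHPController handles damage and signals death, disabling capsule collision and dissolving the mesh before destruction, while timelines drive material hit flashes.
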(event `UpdateState`
  (params (NewState :type "/Game/Blueprints/Monster/EBearState Enum" :default "NewEnumerator0"))
  (bind _charactermovement (`self.CharacterMovement`))
  ;[0.998 1 0 0.5] 몬스터 상태 변경 이벤트
  (if (`|EnumInequality` (`self.State_BP`) "NewEnumerator3")
    (set `self.State_BP` NewState)
    (switch `/Game/Blueprints/Monster/EBearState` (`self.State_BP`)
      (:`NewEnumerator0`
        (set `CharacterMovementComponent.MaxWalkSpeed` 200.0 _charactermovement))
      (:`NewEnumerator1`
        (set `CharacterMovementComponent.MaxWalkSpeed` 400.0 _charactermovement))
      (:`NewEnumerator2`
        (set `CharacterMovementComponent.MaxWalkSpeed` 0.0 _charactermovement :!label _label))
      (:`NewEnumerator3`
        (goto _label)))))

(event `self.ReceiveBeginPlay`
  ;[0 1 0.9749 0.5] 죽음 이벤트에 바인딩
  (add `/Game/Blueprints/Components/BP_HPController.OnDeadEvent` (`self.BP_HPController`) (delegate `ReceiveOnDead`)))

(event `ReceiveOnDead`
  (bind _mesh (`self.Mesh`))
  ;[0 1 0.9749 0.5] 죽음 이벤트에 바인딩
  (`self.UpdateState` "NewEnumerator3")
  (`PrimitiveComponent.SetCollisionEnabled` (`self.CapsuleComponent`) "NoCollision")
  (`KismetSystemLibrary.Delay` 2.0)
  (bind (_direction _dissolve _hitvalue) (`Timeline|DeathEffect` :!via `PlayFromStart`)
    (:`Update`
      (`MeshComponent.SetScalarParameterValueOnMaterials` _mesh "Dissolve" _dissolve)
      (`MeshComponent.SetScalarParameterValueOnMaterials` _mesh "HitValue" _hitvalue))
    (:`Finished`
      (`self.K2_DestroyActor`))))

(event `self.ReceiveActorBeginOverlap`
  (params (OtherActor :type "Actor Object Reference"))
  ; 맞았을 때 피격효과
  (if (`self.ActorHasTag` OtherActor "PlayerWeapon")
    (bind (_direction _hitvalue) (`Timeline|Timeline` :!via `PlayFromStart`)
      (:`Update`
        (`MeshComponent.SetScalarParameterValueOnMaterials` (`self.Mesh`) "HitValue" _hitvalue)))))

(event `self.ReceiveAnyDamage`
  (params (Damage :type "Float (single-precision)") (DamageType :type "DamageType Object Reference") (InstigatedBy :type "Controller Object Reference") (DamageCauser :type "Actor Object Reference"))
  ;[1 0 0.836 0.5] 데미지 처리
  (`/Game/Blueprints/Components/BP_HPController.ReceiveDamage` (`self.BP_HPController`) Damage))

(event `self.PawnSensing.OnSeePawn`
  (params (Pawn :type "Pawn Object Reference"))
  ; 시야감지
  (if (`|EnumEquality` (`self.State_BP`) "NewEnumerator0")
    (if (`self.ActorHasTag` Pawn "Player")
      (`BlackboardComponent.SetValueAsObject` (`AIController.Blackboard` (`AIBlueprintHelperLibrary.GetAIController` self)) (`self.TargetPlayerKey`) Pawn)
      (bind _asbp_character (cast `/Game/Blueprints/Character/BP_Character` Pawn))
      (if (not (`|EnumEquality` (`/Game/Blueprints/Character/BP_Character.State_BP` _asbp_character) "NewEnumerator2"))
        (`self.UpdateState` "NewEnumerator1")))))

(event `self.ReceiveTick`
  (params (DeltaSeconds :type "Float (single-precision)"))
  ;[0.15 0 0.06967 0.5] 간단한 FSM
  (switch `/Game/Blueprints/Monster/EBearState` (`self.State_BP`)
    (:`NewEnumerator0`
      (`self.OnLocomotion`))
    (:`NewEnumerator1`
      (`self.OnChase`))
    (:`NewEnumerator2`
      (`self.OnAttack`))
    (:`NewEnumerator3`
      (`self.OnDead`))))

(fn `OnAttack`
  (bind _asbp_character (cast `/Game/Blueprints/Character/BP_Character` (`BlackboardComponent.GetValueAsObject` (`AIController.Blackboard` (`AIBlueprintHelperLibrary.GetAIController` self)) (`self.TargetPlayerKey`))))
  (if (`|EnumEquality` (`/Game/Blueprints/Character/BP_Character.State_BP` _asbp_character) "NewEnumerator2")
    (`self.UpdateState` "NewEnumerator0")))

(fn `OnChase`
  (bind _asactor (cast `Actor` (`BlackboardComponent.GetValueAsObject` (`AIController.Blackboard` (`AIBlueprintHelperLibrary.GetAIController` self)) (`self.TargetPlayerKey`))))
  (if (> (`KismetMathLibrary.Vector_Distance` (`self.K2_GetActorLocation` _asactor) (`self.K2_GetActorLocation`)) (`PawnSensingComponent.SightRadius` (`self.PawnSensing`)))
    (`self.UpdateState` "NewEnumerator0")))

(fn `OnDead`)

(fn `OnLocomotion`)

(fn `UserConstructionScript`)